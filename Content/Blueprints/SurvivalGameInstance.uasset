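; Game instance for the survival game that owns and manages the runtime UI and the pickable panel widgets.
; Runtime UI is created once for player controller 0 and added to the viewport.
; The pickable panel is created lazily and cached, then shown with Game and UI input, focus and mouse cursor.
; Hiding removes it from the viewport and restores game-only input without the cursor.
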(event `CreateRuntimeUI`
  (`/Engine/EditorBlueprintResources/StandardMacros.IsValid` (`self.RuntimeUI`)
    (:`Is Not Valid`
      (bind _returnvalue (`|CreateWidget` "/Game/UI/RuntimeUI.RuntimeUI_C" (`GameplayStatics.GetPlayerController` 0)))
      (bind _output_get (set `self.RuntimeUI` _returnvalue))
      (`UserWidget.AddToViewport` _output_get 0))))

(event `CreatePickablePanel`
  (bind _returnvalue (`GameplayStatics.GetPlayerController` 0))
  (bind _pickablepanel (`self.PickablePanel`))
  (`/Engine/EditorBlueprintResources/StandardMacros.IsValid` _pickablepanel
    (:`Is Valid`
      (if (not (`Widget.IsInViewport` _pickablepanel))
        (`UserWidget.AddToViewport` (stale _output_get) 0 :!label _label)
        (`WidgetBlueprintLibrary.SetInputMode_GameAndUIEx` _returnvalue (`self.PickablePanel`))
        (set `PlayerController.bShowMouseCursor` true _returnvalue)))
    (:`Is Not Valid`
      (bind _returnvalue_2 (`|CreateWidget` "/Game/UI/PickablePanel.PickablePanel_C" (`GameplayStatics.GetPlayerController` 0)))
      (bind _output_get (set `self.PickablePanel` _returnvalue_2))
      (goto _label))))

(event `HidePickablePanel`
  (bind _returnvalue (`GameplayStatics.GetPlayerController` 0))
  (bind _pickablepanel (`self.PickablePanel`))
  (`/Engine/EditorBlueprintResources/StandardMacros.IsValid` _pickablepanel
    (:`Is Valid`
      (`Widget.RemoveFromParent` _pickablepanel)
      (`WidgetBlueprintLibrary.SetInputMode_GameOnly` _returnvalue)
      (set `PlayerController.bShowMouseCursor` false _returnvalue))))