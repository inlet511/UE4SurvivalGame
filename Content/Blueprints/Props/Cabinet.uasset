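; Cabinet prop that stores items and flags when the survival character is nearby.
; Overlapping AffectArea shows or hides the cabinet panel through the game instance and toggles PlayerNearCabinet on the game mode.
; AddItem and RemoveItem edit the Content array of item slots, matching by type to adjust counts or add and remove entries.
; Both announce changes through added, removed and updated-count calls.
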(event `self.AffectArea.OnComponentBeginOverlap`
  (params (OverlappedComponent :type "PrimitiveComponent Object Reference") (OtherActor :type "Actor Object Reference") (OtherComp :type "PrimitiveComponent Object Reference") (OtherBodyIndex :type Integer) (bFromSweep :type Boolean) (SweepResult :type "HitResult Structure (by ref)"))
  (cast `/Game/Blueprints/SurvivalCharacter` OtherActor)
  (`/Game/Blueprints/SurvivalGameInstance.ShowCabinetPanel` (cast `/Game/Blueprints/SurvivalGameInstance` (`GameplayStatics.GetGameInstance`) :!pure true))
  (set `/Game/Blueprints/SuvivalGameMode.PlayerNearCabinet` true (cast `/Game/Blueprints/SuvivalGameMode` (`GameplayStatics.GetGameMode`) :!pure true)))

(event `self.AffectArea.OnComponentEndOverlap`
  (params (OverlappedComponent :type "PrimitiveComponent Object Reference") (OtherActor :type "Actor Object Reference") (OtherComp :type "PrimitiveComponent Object Reference") (OtherBodyIndex :type Integer))
  (cast `/Game/Blueprints/SurvivalCharacter` OtherActor)
  (`/Game/Blueprints/SurvivalGameInstance.HideCabinetPanel` (cast `/Game/Blueprints/SurvivalGameInstance` (`GameplayStatics.GetGameInstance`) :!pure true))
  (set `/Game/Blueprints/SuvivalGameMode.PlayerNearCabinet` false (cast `/Game/Blueprints/SuvivalGameMode` (`GameplayStatics.GetGameMode`) :!pure true)))

(fn `AddItem`
  (params (NewItem :type "/Game/Blueprints/Struct_ItemSlot Structure"))
  (bind (_type _name _icon _count) (break `/Game/Blueprints/Struct_ItemSlot` NewItem))
  (for (_array_element _array_index) (`self.Content`)
    (if (== _type (`.Type_8_807B3F93417B2DB86693DCBFD8BD3B91` (break `/Game/Blueprints/Struct_ItemSlot` _array_element)))
      (bind _structout (setmembers `/Game/Blueprints/Struct_ItemSlot` :`StructRef` (`|GetArrayItem` (`self.Content`) _array_index) :`Count` (+ _count 1)))
      (`self.AddedItem` _structout)
      (return)))
  (`KismetArrayLibrary.Array_Add` (`self.Content`) NewItem)
  (`self.UpdatedItemCount` (struct))
  (return))

(fn `RemoveItem`
  (params (RemovedItem :type "/Game/Blueprints/Struct_ItemSlot Structure"))
  (bind (_type _name _icon _count) (break `/Game/Blueprints/Struct_ItemSlot` RemovedItem))
  (bind _returnvalue (- _count 1))
  (for (_array_element _array_index) (`self.Content`)
    (if (== _type (`.Type_8_807B3F93417B2DB86693DCBFD8BD3B91` (break `/Game/Blueprints/Struct_ItemSlot` _array_element)))
      (if (== _returnvalue 0)
        (`KismetArrayLibrary.Array_RemoveItem` (`self.Content`))
        (`self.RemovedItem` RemovedItem)
        (else
          (bind _structout (setmembers `/Game/Blueprints/Struct_ItemSlot` :`StructRef` (`|GetArrayItem` (`self.Content`) _array_index) :`Count` _returnvalue))
          (`self.UpdatedItemCount` _structout)))
      (return))))

(fn `UserConstructionScript`)